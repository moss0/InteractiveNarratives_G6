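; Base NPC character that can patrol a spline route, grab or shoot at the player, and start dialogue on interaction.
; Box and sphere overlaps track player range, gating the grab and shoot montages; a grab prints a death message, while only an out-of-range attempt calls the grab-end notification.
; Patrol helpers step along spline points in ping-pong or looping order, alongside enum-based walk speed and a downward trace.
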(event OnComponentBeginOverlap(ShootSphere)
  (params (OverlappedComponent :type Primitive%20Component%20Object%20Reference) (OtherActor :type Actor%20Object%20Reference) (OtherComp :type Primitive%20Component%20Object%20Reference) (OtherBodyIndex :type Integer) (bFromSweep :type Boolean) (SweepResult :type Hit%20Result%20Structure%20%28by%20ref%29))
  (if (== OtherActor (Game|GetPlayerCharacter 0))
    (Variables|Default|SetplayerInShootSphere true)))

(event OnComponentBeginOverlap(Box)
  (params (OverlappedComponent :type Primitive%20Component%20Object%20Reference) (OtherActor :type Actor%20Object%20Reference) (OtherComp :type Primitive%20Component%20Object%20Reference) (OtherBodyIndex :type Integer) (bFromSweep :type Boolean) (SweepResult :type Hit%20Result%20Structure%20%28by%20ref%29))
  (if (== OtherActor (Game|GetPlayerCharacter 0))
    (Variables|Default|SetplayerInGrabBox true)))

(event OnComponentEndOverlap(Box)
  (params (OverlappedComponent :type Primitive%20Component%20Object%20Reference) (OtherActor :type Actor%20Object%20Reference) (OtherComp :type Primitive%20Component%20Object%20Reference) (OtherBodyIndex :type Integer))
  (if (== OtherActor (Game|GetPlayerCharacter 0))
    (Variables|Default|SetplayerInGrabBox false)))

(event OnComponentEndOverlap(ShootSphere)
  (params (OverlappedComponent :type Primitive%20Component%20Object%20Reference) (OtherActor :type Actor%20Object%20Reference) (OtherComp :type Primitive%20Component%20Object%20Reference) (OtherBodyIndex :type Integer))
  (if (== OtherActor (Game|GetPlayerCharacter 0))
    (Variables|Default|SetplayerInShootSphere false)))

(event Custom|ShootAtPlayer
  (if (Variables|Default|GetplayerInShootSphere)
    (Animation|Montage|PlayMontage (Variables|Character|GetMesh) 0)))

(event Custom|TryGrabPlayer
  (if (Variables|Default|GetplayerInGrabBox)
    (Animation|Montage|PlayMontage (Variables|Character|GetMesh) 0
      (:OnCompleted
        _)
      (:OnInterrupted
        _))
    (Variables|Default|SettryGrabPlayerResult true)
    (Development|PrintString "You died")
    (else
      (Variables|Default|SettryGrabPlayerResult false)
      (Default|CallOnTryGrabPlayerEnd (Variables|Default|GettryGrabPlayerResult)))))

(event Custom|UpdateSplineIndex
  (Variables|Patrol|SetpatrolSplineIndex (- (Spline|GetNumberOfSplinePoints (Variables|/Game/Dynamic/Blueprints/AI/BP_PatrolRoute.BP_PatrolRoute_C|GetPatrolRoute (Variables|Patrol|GetpatrolRoute))) 1)))

(event EventBeginPlay
  ;[1 1 1] BeginPlay
  (Utilities|FlowControl|Sequence
    (:then_0
      (CallFunction|UpdateSplineIndex))
    (:then_1
      (if (Variables|Patrol|GetswitchPatrolDirection)
        (Variables|Patrol|SetpatrolDirection -1)
        (else
          (Variables|Patrol|SetpatrolDirection 1))))))

(event EventIncrementPatrolRoute
  (if (and (>= (+ (Variables|Patrol|GetpatrolIndex) (Variables|Patrol|GetpatrolDirection)) 0) (<= (+ (Variables|Patrol|GetpatrolIndex) (Variables|Patrol|GetpatrolDirection)) (Variables|Patrol|GetpatrolSplineIndex)))
    (Variables|Patrol|SetpatrolIndex (+ (Variables|Patrol|GetpatrolIndex) (Variables|Patrol|GetpatrolDirection)))
    (elif (< (+ (Variables|Patrol|GetpatrolIndex) (Variables|Patrol|GetpatrolDirection)) 0)
      (Variables|Patrol|SetpatrolDirection 1)
      (else
        (Variables|Patrol|SetpatrolDirection -1)))))

(event EventIncrementPatrolRouteCircular
  (if (and (>= (+ (Variables|Patrol|GetpatrolIndex) (Variables|Patrol|GetpatrolDirection)) 0) (<= (+ (Variables|Patrol|GetpatrolIndex) (Variables|Patrol|GetpatrolDirection)) (Variables|Patrol|GetpatrolSplineIndex)))
    (Variables|Patrol|SetpatrolIndex (+ (Variables|Patrol|GetpatrolIndex) (Variables|Patrol|GetpatrolDirection)))
    (elif (< (+ (Variables|Patrol|GetpatrolIndex) (Variables|Patrol|GetpatrolDirection)) 0)
      (Variables|Patrol|SetpatrolIndex (Variables|Patrol|GetpatrolSplineIndex))
      (else
        (Variables|Patrol|SetpatrolIndex 0)))))

(event EventInteract
  (Default|StartDialog (Variables|Default|GetBPC_DialogueComponent)))

(fn ConstructionScript)

(fn RaycastDownwards
  (bind _returnvalue (Transformation|GetActorLocation))
  (bind (_outhit _returnvalue_2) (Collision|LineTraceByChannel _returnvalue (+ _returnvalue (* (Math|Vector|GetUpVector (Transformation|GetActorRotation)) (Variables|Default|GetraycastDownSize) -1)) "TraceTypeQuery1" false 0 "ForOneFrame" true "(R=0.000000,G=0.897234,B=1.000000,A=1.000000)" "(R=1.000000,G=0.532573,B=0.000000,A=1.000000)" 1.0))
  (return _outhit _returnvalue_2))

(fn GetBlueprintReference
  (return 0))

(fn GetPatrolRoute
  (return (Variables|Patrol|GetpatrolRoute) (Variables|Patrol|GetpatrolType)))

(fn GetSplinePointasWorldPosition
  (return (Spline|GetLocationatSplinePoint (Variables|/Game/Dynamic/Blueprints/AI/BP_PatrolRoute.BP_PatrolRoute_C|GetPatrolRoute (Variables|Patrol|GetpatrolRoute)) (Variables|Patrol|GetpatrolIndex) "World")))

(fn SetMovementSpeed
  (params (speed :type E_NPC_Base_Speeds%20Enum :default "NewEnumerator0"))
  (bind _output_get (Variables|/Script/Engine.CharacterMovementComponent|SetMaxWalkSpeed (Variables|Character|GetCharacterMovement) (Utilities|Select :Index speed :NewEnumerator0 0.0 :NewEnumerator1 2e+02 :NewEnumerator2 5e+02 :NewEnumerator3 8e+02)))
  (return _output_get))