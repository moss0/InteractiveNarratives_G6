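; BP_DisguiseChecker is a trigger actor that flags whether the player is wearing an acceptable disguise when entering its box.
; It caches the BP_ThirdPersonCharacter at BeginPlay, then on player overlap compares that character's CurrentDisguise against its RequiredDisguises array.
; A match clears IsPlayerNaughty and breaks the loop, while each mismatch sets it.
; The flag is only updated on overlap begin, with no handling on exit.
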(event OnComponentBeginOverlap(Box)
  (params (OverlappedComponent :type Primitive%20Component%20Object%20Reference) (OtherActor :type Actor%20Object%20Reference) (OtherComp :type Primitive%20Component%20Object%20Reference) (OtherBodyIndex :type Integer) (bFromSweep :type Boolean) (SweepResult :type Hit%20Result%20Structure%20%28by%20ref%29))
  (if (== OtherActor (Game|GetPlayerCharacter 0))
    (bind _array_element (Utilities|Array|ForEachLoopwithBreak (Variables|Default|GetrequiredDisguises))
      (:LoopBody
        (if (Utilities|Enum|Equal(Enum) _array_element (Variables|/Game/Dynamic/Blueprints/Player/BP_ThirdPersonCharacter.BP_ThirdPersonCharacter_C|GetcurrentDisguise (Variables|Default|Getplayer)))
          (Variables|/Game/Dynamic/Blueprints/Player/BP_ThirdPersonCharacter.BP_ThirdPersonCharacter_C|SetisPlayerNaughty (Variables|Default|Getplayer) false)
          (CallFunction|BreakLoop)
          (else
            (Variables|/Game/Dynamic/Blueprints/Player/BP_ThirdPersonCharacter.BP_ThirdPersonCharacter_C|SetisPlayerNaughty (Variables|Default|Getplayer) true)))))))

(event Custom|BreakLoop
  (Utilities|Array|ForEachLoopwithBreak (Variables|Default|GetrequiredDisguises)) ; enters at Break
)

(event EventBeginPlay
  (bind _returnvalue (Actor|GetActorOfClass "/Game/Dynamic/Blueprints/Player/BP_ThirdPersonCharacter.BP_ThirdPersonCharacter_C"))
  (Variables|Default|Setplayer _returnvalue))

(fn ConstructionScript)