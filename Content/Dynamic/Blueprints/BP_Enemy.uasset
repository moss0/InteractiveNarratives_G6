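; Enemy character that plays montages to grab or shoot at the player.
; Box and sphere overlaps track whether the player is within grab or shooting range, gating the TryGrabPlayer and ShootAtPlayer events.
; A finished or interrupted grab only sets the result and prints a death message, while the end dispatcher fires only on failure.
; Helper functions provide a downward line trace and map speed tiers to walk speed.
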(event OnComponentBeginOverlap(Sphere)
  (params (OverlappedComponent :type Primitive%20Component%20Object%20Reference) (OtherActor :type Actor%20Object%20Reference) (OtherComp :type Primitive%20Component%20Object%20Reference) (OtherBodyIndex :type Integer) (bFromSweep :type Boolean) (SweepResult :type Hit%20Result%20Structure%20%28by%20ref%29))
  (if (== OtherActor (Game|GetPlayerCharacter 0))
    (Variables|Default|SetplayerInShootSphere true)))

(event OnComponentBeginOverlap(Box)
  (params (OverlappedComponent :type Primitive%20Component%20Object%20Reference) (OtherActor :type Actor%20Object%20Reference) (OtherComp :type Primitive%20Component%20Object%20Reference) (OtherBodyIndex :type Integer) (bFromSweep :type Boolean) (SweepResult :type Hit%20Result%20Structure%20%28by%20ref%29))
  (if (== OtherActor (Game|GetPlayerCharacter 0))
    (Variables|Default|SetplayerInGrabBox true)))

(event OnComponentEndOverlap(Box)
  (params (OverlappedComponent :type Primitive%20Component%20Object%20Reference) (OtherActor :type Actor%20Object%20Reference) (OtherComp :type Primitive%20Component%20Object%20Reference) (OtherBodyIndex :type Integer))
  (if (== OtherActor (Game|GetPlayerCharacter 0))
    (Variables|Default|SetplayerInGrabBox false)))

(event OnComponentEndOverlap(Sphere)
  (params (OverlappedComponent :type Primitive%20Component%20Object%20Reference) (OtherActor :type Actor%20Object%20Reference) (OtherComp :type Primitive%20Component%20Object%20Reference) (OtherBodyIndex :type Integer))
  (if (== OtherActor (Game|GetPlayerCharacter 0))
    (Variables|Default|SetplayerInShootSphere false)))

(event Custom|ShootAtPlayer
  (if (Variables|Default|GetplayerInShootSphere)
    (Animation|Montage|PlayMontage (Variables|Character|GetMesh) 0)))

(event Custom|TryGrabPlayer
  (if (Variables|Default|GetplayerInGrabBox)
    (Animation|Montage|PlayMontage (Variables|Character|GetMesh) 0
      (:OnCompleted
        _)
      (:OnInterrupted
        _))
    (Variables|Default|SetTryGrabPlayerResult true)
    (Development|PrintString "You died")
    (else
      (Variables|Default|SetTryGrabPlayerResult false)
      (Default|CallOnTryGrabPlayerEnd (Variables|Default|GetTryGrabPlayerResult)))))

(fn ConstructionScript)

(fn RaycastDownwards
  (bind _returnvalue (Transformation|GetActorLocation))
  (bind (_outhit _returnvalue_2) (Collision|LineTraceByChannel _returnvalue (+ _returnvalue (* (Math|Vector|GetUpVector (Transformation|GetActorRotation)) (Variables|Default|GetraycastDownSize) -1)) "TraceTypeQuery1" false 0 "ForOneFrame" true "(R=0.000000,G=0.897234,B=1.000000,A=1.000000)" "(R=1.000000,G=0.532573,B=0.000000,A=1.000000)" 1.0))
  (return _outhit _returnvalue_2))

(fn SetMovementSpeed
  (params (speed :type E_EnemySpeeds%20Enum :default "NewEnumerator0"))
  (bind _output_get (Variables|/Script/Engine.CharacterMovementComponent|SetMaxWalkSpeed (Variables|Character|GetCharacterMovement) (Utilities|Select :Index speed :NewEnumerator0 0.0 :NewEnumerator1 2e+02 :NewEnumerator2 5e+02 :NewEnumerator3 8e+02)))
  (return _output_get))