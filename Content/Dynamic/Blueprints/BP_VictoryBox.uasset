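; BP_VictoryBox is a trigger volume that ends the heist when the player reaches it carrying money.
; BeginPlay caches the BP_ThirdPersonCharacter, and the Box overlap checks for the player character and a Money value above zero.
; On success it shows the WB_HeistOver widget, destroys every BP_NPC_Base actor, then loads L_MainMenu after a short delay.
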(event OnComponentBeginOverlap(Box)
  (params (OverlappedComponent :type Primitive%20Component%20Object%20Reference) (OtherActor :type Actor%20Object%20Reference) (OtherComp :type Primitive%20Component%20Object%20Reference) (OtherBodyIndex :type Integer) (bFromSweep :type Boolean) (SweepResult :type Hit%20Result%20Structure%20%28by%20ref%29))
  (if (== OtherActor (Game|GetPlayerCharacter 0))
    (if (> (Variables|/Game/Dynamic/Blueprints/Player/BP_ThirdPersonCharacter.BP_ThirdPersonCharacter_C|Getmoney (Variables|Default|Getplayer)) 0.0)
      (bind _returnvalue (UserInterface|CreateWidget "/Game/Dynamic/Blueprints/UI/WB_HeistOver.WB_HeistOver_C"))
      (UserInterface|Viewport|AddtoViewport _returnvalue 5)
      (bind _outactors (Actor|GetAllActorsOfClass "/Game/Dynamic/Blueprints/AI/BP_NPC_Base.BP_NPC_Base_C"))
      (for _array_element _outactors
        (Actor|DestroyActor _array_element))
      (Utilities|FlowControl|Delay 1e+01)
      (Game|OpenLevel(byName) "L_MainMenu"))))

(event EventBeginPlay
  (bind _returnvalue (Actor|GetActorOfClass "/Game/Dynamic/Blueprints/Player/BP_ThirdPersonCharacter.BP_ThirdPersonCharacter_C"))
  (Variables|Default|Setplayer _returnvalue))

(fn ConstructionScript)