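; BP_BaseCollectable is a base class for collectable actors that the player picks up by interacting with them.
; Interact runs StartInteraction, which checks CanBePickedUp (true by default) before calling OnPickup.
; OnPickup plays an optional pickup sound at the static mesh location and destroys the actor.
; BeginPlay caches a reference to the BP_ThirdPersonCharacter player.
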(event Custom|OnPickup
  (bind _pickupsound (Variables|Default|GetpickupSound)
    (:then
      (Audio|PlaySoundatLocation _pickupsound (Transformation|GetWorldLocation (Variables|Default|GetStaticMesh)) "0, 0, 0" 1.0 1.0 0.0 0 0 0 0))
    (:else
      _))
  (Actor|DestroyActor))

(event Custom|StartInteraction
  (bind _canbepickedup (CallFunction|CanbePickedUp))
  (if _canbepickedup
    (CallFunction|OnPickup)))

(event EventInteract
  (CallFunction|StartInteraction))

(event EventBeginPlay
  (bind _returnvalue (Actor|GetActorOfClass "/Game/Dynamic/Blueprints/Player/BP_ThirdPersonCharacter.BP_ThirdPersonCharacter_C"))
  (Variables|Default|Setplayer _returnvalue))

(fn ConstructionScript)

(fn CanbePickedUp
  (return true))