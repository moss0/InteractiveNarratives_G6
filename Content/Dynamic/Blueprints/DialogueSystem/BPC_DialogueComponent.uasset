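; BPC_DialogueComponent is a component that starts a conversation between its NPC and the player, using a dialogue data table.
; StartDialog stores the given starting line ID, checks that the table is valid and lazily caches the GI_FGCT4007 game instance.
; It then passes itself, the line ID, the table and the player character to the game instance's BeginConversation.
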(event EventBeginPlay)

(event EventTick
  (params (DeltaSeconds :type Float%20%28single-precision%29)))

(fn StartDialog
  (params (StartingDialogID :type Integer))
  (Variables|Default|SetDefaultStartlingLineID StartingDialogID)
  (Utilities|IsValid (Variables|Default|GetDT_Dialogue)
    (:Is%20Valid
      (Utilities|IsValid (Variables|Default|GetGameInstance)
        (:Is%20Valid
          _)
        (:Is%20Not%20Valid
          (bind _asgi_fgct4007 (Utilities|Casting|CastToGI_FGCT4007 (Game|GetGameInstance)))
          (bind _output_get (Variables|Default|SetGameInstance _asgi_fgct4007))))
      (Default|BeginConversation _output_get self (Variables|Default|GetDefaultStartlingLineID) (Variables|Default|GetDT_Dialogue) (Game|GetPlayerCharacter 0)))))